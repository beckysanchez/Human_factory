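; BP_ventila is a window actor that reacts to repaired boxes reported through its RegistrarCajaReparada event.
; Each call increments a repaired-box counter and updates the VentilaAbierta flag.
; Below three boxes it flags the window open and plays the AbrirVentanilla timeline, which sets the Ventila component's relative rotation through a yaw lerp.
; From the third box onward it only clears the flag, without playing or reversing the timeline.
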(event Custom|RegistrarCajaReparada
  (Variables|Default|SetcajasReparadas (+ (Variables|Default|GetcajasReparadas) 1.0))
  (if (>= (Variables|Default|GetcajasReparadas) 3.0)
    (Variables|Default|SetventilaAbierta? false)
    (else
      (Variables|Default|SetventilaAbierta? true)
      (Timeline|abrirVentanilla Play
        (:Update
          (Transformation|SetRelativeRotation (Variables|Default|Getventila) (Math|Rotator|Lerp(Rotator) "0, 0, 0" "90.000000,0.000000,0.000000" 0.0) false false))))))

(event EventBeginPlay)

(event Collision|EventActorBeginOverlap
  (params (OtherActor :type Actor%20Object%20Reference)))

(event EventTick
  (params (DeltaSeconds :type Float%20%28single-precision%29)))

(fn ConstructionScript)