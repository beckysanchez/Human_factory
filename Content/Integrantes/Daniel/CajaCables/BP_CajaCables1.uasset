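; BP_CajaCables1 is a cable box that a BP_CharacterMouse player repairs by staying nearby while repairing.
; A Box overlap tracks the nearby player, and Tick adds a fixed, frame-rate-dependent progress step, shown on that player's progress bar.
; On completion it hides the bar, clears the player's repairing flag and registers the repair with AsBPVentila, a reference this graph never assigns.
; BeginPlay caches BP_GameModeJuego, otherwise unused here.
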(event OnComponentBeginOverlap(Box)
  (params (OverlappedComponent :type Primitive%20Component%20Object%20Reference) (OtherActor :type Actor%20Object%20Reference) (OtherComp :type Primitive%20Component%20Object%20Reference) (OtherBodyIndex :type Integer) (bFromSweep :type Boolean) (SweepResult :type Hit%20Result%20Structure%20%28by%20ref%29))
  (bind _asbp_character_mouse (Utilities|Casting|CastToBP_CharacterMouse OtherActor))
  (Variables|Default|SetJugadorActual _asbp_character_mouse)
  (Variables|Default|SetEstaCerca true))

(event OnComponentEndOverlap(Box)
  (params (OverlappedComponent :type Primitive%20Component%20Object%20Reference) (OtherActor :type Actor%20Object%20Reference) (OtherComp :type Primitive%20Component%20Object%20Reference) (OtherBodyIndex :type Integer))
  (Variables|Default|SetEstaCerca false)
  (Variables|Default|SetJugadorActual 0))

(event EventTick
  (params (DeltaSeconds :type Float%20%28single-precision%29))
  (bind _as_bp_ventila (Variables|Default|GetAs%20BP%20Ventila))
  (if (Variables|Default|GetEstaCerca)
    (if (Utilities|IsValid (Variables|Default|GetJugadorActual))
      (if (Variables|/Game/Integrantes/Daniel/BP_CharacterMouse.BP_CharacterMouse_C|GetReparando? (Variables|Default|GetJugadorActual))
        (if (not (Variables|Default|GetcajaReparada?))
          (bind _output_get (Variables|Default|SetProgreso (+ (Variables|Default|GetProgreso) 0.005)))
          (Progress|SetPercent (Variables|/Game/Integrantes/Daniel/Interfaz/WBP_BarraReparacion.WBP_BarraReparacion_C|GetProgressBar_116 (Variables|/Game/Integrantes/Daniel/BP_CharacterMouse.BP_CharacterMouse_C|GetMiBarra (Variables|Default|GetJugadorActual))) _output_get)
          (Development|PrintString (Utilities|String|ToString(Float) _output_get))
          (if (>= (Variables|Default|GetProgreso) 1.0)
            (Variables|Default|SetCajaReparada? true)
            (Widget|SetVisibility (Variables|/Game/Integrantes/Daniel/BP_CharacterMouse.BP_CharacterMouse_C|GetMiBarra (Variables|Default|GetJugadorActual)) "Hidden")
            (Variables|/Game/Integrantes/Daniel/BP_CharacterMouse.BP_CharacterMouse_C|SetReparando? (Variables|Default|GetJugadorActual) false)
            (Utilities|IsValid _as_bp_ventila
              (:Is%20Valid
                (Default|RegistrarCajaReparada _as_bp_ventila)
                (Development|PrintString "es valido" true true "(R=0.532455,G=0.000000,B=1.000000,A=1.000000)"))
              (:Is%20Not%20Valid
                (Development|PrintString "no es valdo")))))))))

(event Collision|EventActorBeginOverlap
  (params (OtherActor :type Actor%20Object%20Reference)))

(event EventBeginPlay
  (bind _asbp_game_mode_juego (Utilities|Casting|CastToBP_GameModeJuego (Game|GetGameMode)))
  (Variables|Default|SetAs%20BP%20Game%20Mode%20Juego _asbp_game_mode_juego))

(fn ConstructionScript)