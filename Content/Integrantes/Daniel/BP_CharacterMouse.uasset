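; Player mouse character for a multiplayer game against scientists, with movement, health and a death montage before destruction.
; Right-click bites, stunning a scientist via sphere trace, and while held at an unrepaired cable box flags repairing and shows a progress widget.
; A potion can be carried on a socket, dropped, drunk to hide the mouse briefly, or thrown as a projectile along camera aim.
; Actions route through server events, with multicasts for potion and death effects.
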(event OnComponentBeginOverlap(CapsuleComponent)
  (params (OverlappedComponent :type Primitive%20Component%20Object%20Reference) (OtherActor :type Actor%20Object%20Reference) (OtherComp :type Primitive%20Component%20Object%20Reference) (OtherBodyIndex :type Integer) (bFromSweep :type Boolean) (SweepResult :type Hit%20Result%20Structure%20%28by%20ref%29))
  (bind _asbp_caja_cables_1 (Utilities|Casting|CastToBP_CajaCables1 OtherActor))
  (Variables|Default|SetEnCaja? true)
  (Variables|Default|SetcajaActual _asbp_caja_cables_1))

(event OnComponentEndOverlap(CapsuleComponent)
  (params (OverlappedComponent :type Primitive%20Component%20Object%20Reference) (OtherActor :type Actor%20Object%20Reference) (OtherComp :type Primitive%20Component%20Object%20Reference) (OtherBodyIndex :type Integer))
  (Utilities|Casting|CastToBP_CajaCables1 OtherActor)
  (Variables|Default|SetEnCaja? false)
  (Variables|Default|SetcajaActual 0)
  (Variables|Default|SetReparando? false))

(event Custom|PeticionMuerte_Server
  ;[0.15 0.15 0.15 0.5] Muerte
  (CallFunction|EjecutarMuerteMulticast))

(event Custom|PeticionLanzar_Server
  (params (direccion :type Vector))
  (if (Variables|Default|GetTienePocion)
    (Variables|Default|SetTienePocion false)
    (CallFunction|EjecutarLanzarMulticast direccion)))

(event Custom|Multicas_TomarPocion
  ;[0.15 0.15 0.15 0.5] Tomar Pocion Q
  (Transformation|DetachFromActor (Variables|Default|GetPotionRef) "KeepWorld" "KeepWorld" "KeepRelative")
  (Rendering|SetActorHiddenInGame (Variables|Default|GetPotionRef) true)
  (Rendering|SetActorHiddenInGame true)
  (Utilities|FlowControl|Delay 5.0)
  (Rendering|SetActorHiddenInGame false))

(event Custom|EjecutarLanzar_Multicast
  (params (direccion :type Vector))
  (Variables|Default|SetVarDireccion (* direccion (Math|Conversions|ToVector(Float) 2e+03)))
  (Pawn|Components|CharacterMovement|DisableMovement (Variables|Character|GetCharacterMovement))
  (Animation|Montage|PlayMontage (Variables|Character|GetMesh) "/Game/Integrantes/Daniel/Mouse/Animations/MouseLanzar_Montage.MouseLanzar_Montage"
    (:OnCompleted
      (Pawn|Components|CharacterMovement|SetMovementMode (Variables|Character|GetCharacterMovement) "MOVE_Walking" 0)
      (Utilities|IsValid (Variables|Default|GetPotionRef)
        (:Is%20Valid
          (Components|Activation|SetActive (Variables|/Game/Integrantes/Jairo/powerUps/poti-invisible/BP_Pocion_Invisibilidad.BP_Pocion_Invisibilidad_C|GetdeteccionCientifico (Variables|Default|GetPotionRef)) true false)
          (Transformation|DetachFromActor (Variables|Default|GetPotionRef) "KeepWorld" "KeepWorld" "KeepWorld")
          (Variables|/Game/Integrantes/Jairo/powerUps/poti-invisible/BP_Pocion_Invisibilidad.BP_Pocion_Invisibilidad_C|SetfueLanzada (Variables|Default|GetPotionRef) true)
          (Transformation|SetActorLocation (Variables|Default|GetPotionRef) (+ (Transformation|GetActorLocation) "0.000000,0.000000,50.000000") false false)
          (Collision|SetActorEnableCollision (Variables|Default|GetPotionRef) true)
          (Components|Activation|Activate (Variables|/Game/Integrantes/Jairo/powerUps/poti-invisible/BP_Pocion_Invisibilidad.BP_Pocion_Invisibilidad_C|GetPocionProyectil (Variables|Default|GetPotionRef)) false)
          (Variables|/Script/Engine.MovementComponent|SetVelocity (Variables|/Game/Integrantes/Jairo/powerUps/poti-invisible/BP_Pocion_Invisibilidad.BP_Pocion_Invisibilidad_C|GetPocionProyectil (Variables|Default|GetPotionRef)) (Variables|Default|GetVarDireccion))
          (Variables|Default|SetPotionRef 0))))))

(event Custom|Server_AturdirCientifico
  (bind _returnvalue (Transformation|GetActorLocation))
  ;[0.15 0.15 0.15 0.5] Daño de Mordida
  (bind (_outhit _returnvalue_2) (Collision|SphereTraceByChannel _returnvalue (+ (* (Transformation|GetActorForwardVector) 1.5e+02) _returnvalue) 4e+01 "TraceTypeQuery2" false 0 "ForDuration"))
  (if _returnvalue_2
    (bind _asbp_character_cientifico (Utilities|Casting|CastToBP_CharacterCientifico (.HitActor (Collision|BreakHitResult _outhit))))
    (Default|ServerRecibirMordida _asbp_character_cientifico)))

(event Custom|PeticionMorder_Server
  ;[0.15 0.15 0.15 0.5] Animación Lanzar y morder
  (CallFunction|EjecutarMorderServer))

(event Custom|EjecutarMorder_Server
  ;[0.15 0.15 0.15 0.5] Animación Lanzar y morder
  (Pawn|Components|CharacterMovement|DisableMovement (Variables|Character|GetCharacterMovement))
  (Animation|Montage|PlayMontage (Variables|Character|GetMesh) "/Game/Integrantes/Daniel/Mouse/Animations/MouseMordida_Montage.MouseMordida_Montage"
    (:OnCompleted
      (Pawn|Components|CharacterMovement|SetMovementMode (Variables|Character|GetCharacterMovement) "MOVE_Walking" 0))))

(event Custom|EjecutarMuerte_Multicast
  ;[0.15 0.15 0.15 0.5] Muerte
  (Pawn|Components|CharacterMovement|DisableMovement (Variables|Character|GetCharacterMovement))
  (Animation|Montage|PlayMontage (Variables|Character|GetMesh) "/Game/Integrantes/Daniel/Mouse/Animations/MouseDying_Montage.MouseDying_Montage"
    (:then
      (Utilities|FlowControl|Delay 5.0)
      (Actor|DestroyActor))))

(event Custom|Server_RecogerPocion
  ;[0.15 0.15 0.15 0.5] Recoger Pocion E
  (if (Variables|Default|GetTienePocion)
    (Variables|Default|SetTienePocion false)
    (else
      (Utilities|IsValid (Variables|Default|GetPotionRef)
        (:Is%20Valid
          (Variables|Default|SetTienePocion true)))))
  (CallFunction|MulticastRecogerPocion))

(event Custom|Multicast_RecogerPocion
  (bind _potionref (Variables|Default|GetPotionRef))
  (bind _potionref_2 (Variables|Default|GetPotionRef))
  (bind _potionref_3 (Variables|Default|GetPotionRef))
  ;[0.15 0.15 0.15 0.5] Recoger Pocion E
  (if (Variables|Default|GetTienePocion)
    (Collision|SetActorEnableCollision _potionref_3 false)
    (Transformation|AttachComponentToComponent _potionref_3 (Variables|Character|GetMesh) "PotionSocket" "SnapToTarget" "SnapToTarget" "KeepRelative" true)
    (Rendering|SetActorHiddenInGame _potionref_2 false)
    (Utilities|IsValid _potionref_2
      (:Is%20Valid
        (Components|Activation|SetActive (Variables|/Game/Integrantes/Jairo/powerUps/poti-invisible/BP_Pocion_Invisibilidad.BP_Pocion_Invisibilidad_C|GetdeteccionCientifico _potionref_2) false false)))
    (else
      (Transformation|DetachFromActor (Variables|Default|GetPotionRef) "KeepWorld" "KeepWorld" "KeepRelative")
      (Rendering|SetActorHiddenInGame (Variables|Default|GetPotionRef) false)
      (Transformation|SetActorLocation _potionref (+ (Transformation|GetActorLocation self) "0.000000,0.000000,-70.000000") false false)
      (Collision|SetActorEnableCollision _potionref false))))

(event Custom|Server_TomarPocion
  ;[0.15 0.15 0.15 0.5] Tomar Pocion Q
  (if (Variables|Default|GetTienePocion)
    (CallFunction|MulticasTomarPocion)
    (Actor|DestroyActor (Variables|Default|GetPotionRef))
    (Variables|Default|SetTienePocion false)
    (Variables|Default|SetPotionRef 0)))

(event EventBeginPlay
  (bind _returnvalue (UserInterface|CreateWidget "/Game/Integrantes/Daniel/Interfaz/WBP_BarraReparacion.WBP_BarraReparacion_C"))
  (Variables|Default|SetMiBarra _returnvalue)
  (UserInterface|Viewport|AddtoViewport _returnvalue 0)
  (Widget|SetVisibility (Variables|Default|GetMiBarra) "Hidden"))

(event Game|Damage|EventAnyDamage
  (params (Damage :type Float%20%28single-precision%29) (DamageType :type Damage%20Type%20Object%20Reference) (InstigatedBy :type Controller%20Object%20Reference) (DamageCauser :type Actor%20Object%20Reference))
  (bind _output_get (Variables|Default|SetHealth (- (Variables|Default|GetHealth) Damage)))
  (if (<= _output_get 0.0)
    (CallFunction|PeticionMuerteServer)
    (else
      (Development|PrintString (Utilities|String|ToString(Float) _output_get)))))

(event Input|ActionEvents|InputActionSaltoCharacterMouse
  (params (Key :type Key%20Structure :default "None"))
  (:Pressed
    (Character|Jump))
  (:Released
    (Character|StopJumping)))

(event Input|AxisEvents|InputAxisMovimiento-Adelante-Atras
  (params (AxisValue :type Float%20%28single-precision%29))
  ;[0.15 0.15 0.15 0.5] Tecla W/S
  (Pawn|Input|AddMovementInput (Math|Vector|GetForwardVector (Math|Rotator|MakeRotator 0.0 0.0 (.yaw (Pawn|GetControlRotation :!class /Script/Engine.Pawn)))) AxisValue false))

(event Input|AxisEvents|InputAxisMovimiento-Izq-Der
  (params (AxisValue :type Float%20%28single-precision%29))
  (bind _returnvalue (Pawn|GetControlRotation :!class /Script/Engine.Pawn))
  ;[0.15 0.15 0.15 0.5] Tecla A/D
  (Pawn|Input|AddMovementInput (Math|Vector|GetRightVector (Math|Rotator|MakeRotator (.roll _returnvalue) 0.0 (.yaw _returnvalue))) AxisValue false))

(event Input|AxisEvents|InputAxisCamaraRaton-Arrib-Abajo
  (params (AxisValue :type Float%20%28single-precision%29))
  (Pawn|Input|AddControllerPitchInput AxisValue))

(event Input|AxisEvents|InputAxisCamaraRaton-Izq-Der
  (params (AxisValue :type Float%20%28single-precision%29))
  (Pawn|Input|AddControllerYawInput AxisValue))

(event Input|MouseEvents|RightMouseButton
  (params (Key :type Key%20Structure :default "None"))
  (:Pressed
    (Utilities|FlowControl|Sequence
      (:then_0
        ;[0.15 0.15 0.15 0.5] Daño de Mordida
        (CallFunction|ServerAturdirCientifico))
      (:then_1
        (if (Variables|Default|GetEnCaja?)
          (if (Utilities|IsValid (Variables|Default|GetcajaActual))
            (if (Variables|/Game/Integrantes/Daniel/CajaCables/BP_CajaCables1.BP_CajaCables1_C|GetcajaReparada? (Variables|Default|GetcajaActual))
              (Development|PrintText "Caja Reparada" true true "(R=1.000000,G=0.766622,B=0.027320,A=1.000000)")
              (else
                (Widget|SetVisibility (Variables|Default|GetMiBarra) "Visible")
                (Variables|Default|SetReparando? true))))))))
  (:Released
    (Widget|SetVisibility (Variables|Default|GetMiBarra) "Hidden")
    (Variables|Default|SetReparando? false)))

(event Input|MouseEvents|LeftMouseButton
  (params (Key :type Key%20Structure :default "None"))
  (:Pressed
    (CallFunction|PeticionLanzarServer (Math|Vector|GetForwardVector (Camera|GetCameraRotation (Game|GetPlayerCameraManager 0))))))

(event Input|KeyboardEvents|1
  (params (Key :type Key%20Structure :default "None"))
  ;[0.15 0.15 0.15 0.5] Muerte
  (:Pressed
    (CallFunction|PeticionMuerteServer)))

(event Input|MouseEvents|RightMouseButton
  (params (Key :type Key%20Structure :default "None"))
  ;[0.15 0.15 0.15 0.5] Animación Lanzar y morder
  (:Pressed
    (CallFunction|PeticionMorderServer)))

(event Input|KeyboardEvents|E
  (params (Key :type Key%20Structure :default "None"))
  ;[0.15 0.15 0.15 0.5] Recoger Pocion E
  (:Pressed
    (CallFunction|ServerRecogerPocion)))

(event Input|KeyboardEvents|Q
  (params (Key :type Key%20Structure :default "None"))
  ;[0.15 0.15 0.15 0.5] Tomar Pocion Q
  (:Pressed
    (CallFunction|ServerTomarPocion)))

(fn ConstructionScript)

(fn SetPotionRef
  (params (Pocion :type BP%20Pocion%20Invisibilidad%20Object%20Reference))
  (Variables|Default|SetPotionRef Pocion))