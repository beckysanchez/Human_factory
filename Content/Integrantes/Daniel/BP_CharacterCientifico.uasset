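; Networked player character for the scientist, who fights mouse characters with a toggled pistol and a stomp.
; Input calls server events: aimed shots apply damage via a line trace from player 0's camera, even on the server.
; The multicast stomp plays an animation and briefly enables a collision that damages overlapping mice.
; A bite event lowers the gun, freezes movement and shows a client dizzy filter for a few seconds.
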(event OnComponentBeginOverlap(ColisionPisada)
  (params (OverlappedComponent :type Primitive%20Component%20Object%20Reference) (OtherActor :type Actor%20Object%20Reference) (OtherComp :type Primitive%20Component%20Object%20Reference) (OtherBodyIndex :type Integer) (bFromSweep :type Boolean) (SweepResult :type Hit%20Result%20Structure%20%28by%20ref%29))
  ;[0.15 0.15 0.15 0.5] Pisada
  (bind _asbp_character_mouse (Utilities|Casting|CastToBP_CharacterMouse OtherActor))
  (Game|Damage|ApplyDamage _asbp_character_mouse 25.0 0 self))

(event Custom|Server_ToggleAim
  (Variables|Default|SetIsAiming (not (Variables|Default|GetIsAiming)))
  (Variables|Default|SetGunVisible (Variables|Default|GetIsAiming))
  (Transformation|AttachComponentToComponent (Variables|Default|GetPistola) (Variables|Character|GetMesh) "GunSocket" "SnapToTarget" "SnapToTarget" "KeepRelative" true)
  (Rendering|SetVisibility (Variables|Default|GetPistola) (Variables|Default|GetGunVisible) false)
  (Development|PrintString "E Presionada"))

(event Custom|Server_Disparar
  (CallFunction|Disparar))

(event Custom|Server_RecibirMordida
  ;[0.15 0.15 0.15 0.5] RecibirMordida
  (Variables|Default|SetIsAiming false)
  (Variables|Default|SetGunVisible false)
  (Variables|/Script/Engine.CharacterMovementComponent|SetMaxWalkSpeed (Variables|Character|GetCharacterMovement) 0.0)
  (CallFunction|ClientEfectoMareado)
  (Utilities|FlowControl|Delay 7.0)
  (CallFunction|ClientQuitarMareado)
  (Variables|/Script/Engine.CharacterMovementComponent|SetMaxWalkSpeed (Variables|Character|GetCharacterMovement) 8e+02))

(event Custom|Client_EfectoMareado
  ;[0.15 0.15 0.15 0.5] RecibirMordida
  (Variables|/Script/Engine.PostProcessComponent|SetbEnabled (Variables|Default|GetFiltroBorracho) true))

(event Custom|Client_QuitarMareado
  ;[0.15 0.15 0.15 0.5] RecibirMordida
  (Variables|/Script/Engine.PostProcessComponent|SetbEnabled (Variables|Default|GetFiltroBorracho) false))

(event Custom|Server_Pisoton
  ;[0.15 0.15 0.15 0.5] Pisada
  (CallFunction|MulticastPisoton)
  (Components|Animation|PlayAnimation (Variables|Character|GetMesh) "/Game/Integrantes/Daniel/Cientifico/Animations/Stomping.Stomping" false)
  (Utilities|FlowControl|Delay 0.4)
  (Collision|SetCollisionEnabled (Variables|Default|GetColisionPisada) "QueryOnly")
  (Utilities|FlowControl|Delay 0.1)
  (Collision|SetCollisionEnabled (Variables|Default|GetColisionPisada) "NoCollision")
  (Utilities|FlowControl|Delay 1.2)
  (Components|Animation|SetAnimationMode (Variables|Character|GetMesh) "AnimationBlueprint" true))

(event Custom|Multicast_Pisoton
  ;[0.15 0.15 0.15 0.5] Pisada
  (Components|Animation|PlayAnimation (Variables|Character|GetMesh) "/Game/Integrantes/Daniel/Cientifico/Animations/Stomping.Stomping" false)
  (Utilities|FlowControl|Delay 0.4)
  (Collision|SetCollisionEnabled (Variables|Default|GetColisionPisada) "QueryOnly")
  (Utilities|FlowControl|Delay 0.1)
  (Collision|SetCollisionEnabled (Variables|Default|GetColisionPisada) "NoCollision")
  (Utilities|FlowControl|Delay 1.2)
  (Components|Animation|SetAnimationMode (Variables|Character|GetMesh) "AnimationBlueprint" true))

(event Input|EnhancedActionEvents|EnhancedInputActionIA_AimToggle
  (params (ActionValue :type Boolean) (ElapsedSeconds :type Float%20%28double-precision%29) (TriggeredSeconds :type Float%20%28double-precision%29) (InputAction :type Input%20Action%20Object%20Reference :default "/Game/Input/Actions/IA_AimToggle.IA_AimToggle"))
  (:Started
    (CallFunction|ServerToggleAim)))

(event Input|EnhancedActionEvents|EnhancedInputActionIA_Shoot
  (params (ActionValue :type Boolean) (ElapsedSeconds :type Float%20%28double-precision%29) (TriggeredSeconds :type Float%20%28double-precision%29) (InputAction :type Input%20Action%20Object%20Reference :default "/Game/Input/Actions/IA_Shoot.IA_Shoot"))
  (:Started
    (if (Variables|Default|GetIsAiming)
      (CallFunction|ServerDisparar))))

(event EventPossessed
  (params (NewController :type Controller%20Object%20Reference))
  (bind _asplayer_controller (Utilities|Casting|CastToPlayerController NewController))
  (Input|AddMappingContext (PlayerController|LocalPlayerSubsystems|GetEnhancedInputLocalPlayerSubsystem _asplayer_controller) "/Game/Input/IMC_Default.IMC_Default" 0 "(bIgnoreAllPressedKeysUntilRelease=True,bForceImmediately=False,bNotifyUserSettings=False)")
  (if (Pawn|IsLocallyControlled)
    (bind _foundwidgets (Widget|GetAllWidgetsOfClass "/Game/FirstPerson/Blueprints/HealthBox.HealthBox_C" true))
    (for _array_element _foundwidgets
      (Widget|RemovefromParent _array_element))))

(event EventBeginPlay
  (bind _destruirpocion (Variables|Default|GetDestruirPocion))
  (bind _returnvalue (UserInterface|CreateWidget "/Game/Integrantes/Alex/WBP_Crosshair.WBP_Crosshair_C"))
  (UserInterface|Viewport|AddtoViewport _returnvalue 0)
  (if (Variables|/Game/Integrantes/Jairo/powerUps/poti-invisible/BP_Pocion_Invisibilidad.BP_Pocion_Invisibilidad_C|GetGolpeo _destruirpocion)
    (Default|ServerDestruir _destruirpocion)
    (Variables|/Game/Integrantes/Jairo/powerUps/poti-invisible/BP_Pocion_Invisibilidad.BP_Pocion_Invisibilidad_C|SetGolpeo (Variables|Default|GetDestruirPocion) false)))

(event Input|AxisEvents|InputAxisMovimiento-Adelante-Atras
  (params (AxisValue :type Float%20%28single-precision%29))
  ;[0.15 0.15 0.15 0.5] Tecla W/S
  (Pawn|Input|AddMovementInput (Math|Vector|GetForwardVector (Math|Rotator|MakeRotator 0.0 0.0 (.yaw (Pawn|GetControlRotation :!class /Script/Engine.Pawn)))) AxisValue false))

(event Input|AxisEvents|InputAxisMovimiento-Izq-Der
  (params (AxisValue :type Float%20%28single-precision%29))
  (bind _returnvalue (Pawn|GetControlRotation :!class /Script/Engine.Pawn))
  ;[0.15 0.15 0.15 0.5] Tecla A/D
  (Pawn|Input|AddMovementInput (Math|Vector|GetRightVector (Math|Rotator|MakeRotator (.roll _returnvalue) 0.0 (.yaw _returnvalue))) AxisValue false))

(event Input|AxisEvents|InputAxisCamaraRaton-Arrib-Abajo
  (params (AxisValue :type Float%20%28single-precision%29))
  ;[0.15 0.15 0.15 0.5] Camara
  (Pawn|Input|AddControllerPitchInput AxisValue))

(event Input|AxisEvents|InputAxisCamaraRaton-Izq-Der
  (params (AxisValue :type Float%20%28single-precision%29))
  ;[0.15 0.15 0.15 0.5] Camara
  (Pawn|Input|AddControllerYawInput AxisValue))

(event Input|KeyboardEvents|Q
  (params (Key :type Key%20Structure :default "None"))
  ;[0.15 0.15 0.15 0.5] Pisada
  (:Pressed
    (CallFunction|ServerPisoton)))

(fn ConstructionScript)

(fn Disparar
  (bind _returnvalue (Game|GetPlayerCameraManager 0))
  (bind _returnvalue_2 (Camera|GetCameraLocation _returnvalue))
  (bind (_outhit _returnvalue_3) (Collision|LineTraceByChannel _returnvalue_2 (+ _returnvalue_2 (* (Math|Vector|GetForwardVector (Camera|GetCameraRotation _returnvalue)) (Math|Conversions|ToVector(Float) 6e+04))) "TraceTypeQuery1" false 0 "None"))
  (Game|Damage|ApplyDamage (.HitActor (Collision|BreakHitResult _outhit)) 1e+02 0 0))