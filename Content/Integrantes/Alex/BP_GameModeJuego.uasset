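; Game mode that gives each joining player a character, making the first player the scientist and every later one the mouse.
; PostLogin increments a player counter, spawns the matching character at a PlayerStart and has the new controller possess it.
; Start points come from fixed indices in the GetAllActorsOfClass result, so placement depends on array order and all mouse players share one start.
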(event EventBeginPlay)

(event EventTick
  (params (DeltaSeconds :type Float%20%28single-precision%29)))

(event EventPostLogin
  (params (NewPlayer :type Player%20Controller%20Object%20Reference))
  (Variables|Default|SetContadorJugadores (+ 1 (Variables|Default|GetContadorJugadores)))
  (bind _outactors (Actor|GetAllActorsOfClass "/Script/Engine.PlayerStart"))
  (if (== (Variables|Default|GetContadorJugadores) 1)
    (bind _returnvalue (Game|SpawnActorfromClass "/Game/Integrantes/Daniel/BP_CharacterCientifico.BP_CharacterCientifico_C" (Transformation|GetActorTransform (Utilities|Array|Get(acopy) _outactors 1)) "Undefined" "MultiplyWithRoot" 0 0))
    (Pawn|Possess NewPlayer _returnvalue)
    (else
      (bind _returnvalue_2 (Game|SpawnActorfromClass "/Game/Integrantes/Daniel/BP_CharacterMouse.BP_CharacterMouse_C" (Transformation|GetActorTransform (Utilities|Array|Get(acopy) _outactors)) "Undefined" "MultiplyWithRoot" 0 0))
      (Pawn|Possess NewPlayer _returnvalue_2))))

(fn ConstructionScript)